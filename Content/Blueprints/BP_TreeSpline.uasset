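; BP_TreeSpline is a construction-time placement actor that puts instances of a tree mesh along a spline.
; The construction script derives spacing from the mesh's bounding-box X size plus an offset, then adds unrotated, unit-scale instances to an InstancedStaticMesh at those distances in local space.
; The loop's last index is spacing divided by spline length, floored, an inverted ratio that does not fill the spline.
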(event EventBeginPlay)

(event Collision|EventActorBeginOverlap
  (params (OtherActor :type Actor%20Object%20Reference)))

(event EventTick
  (params (DeltaSeconds :type Float%20%28single-precision%29)))

(fn ConstructionScript
  (bind _spline (Variables|Default|GetSpline))
  (bind _treemesh (Variables|Default|GetTreeMesh))
  (bind _returnvalue (StaticMesh|GetBoundingBox _treemesh))
  (Components|StaticMesh|SetStaticMesh (Variables|Default|GetInstancedStaticMesh) (Variables|Default|GetTreeMesh))
  (bind _output_get (Variables|Default|SetSpacing (+ (.X (Math|Vector|BreakVector (- (.max _returnvalue) (.min _returnvalue)))) (Variables|Default|GetOffset))))
  (bind _output_get_2 (Variables|Default|SetInstancesNumber (Math|Float|Floor (/ _output_get (Spline|GetSplineLength _spline)))))
  (for _index (range 0 _output_get_2)
    (Components|InstancedStaticMesh|AddInstance (Variables|Default|GetInstancedStaticMesh) (Math|Transform|MakeTransform (Spline|GetLocationatDistanceAlongSpline _spline (* _index (Variables|Default|GetSpacing)) "Local")) false)))