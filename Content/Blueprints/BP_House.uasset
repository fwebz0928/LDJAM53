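; BP_House is a delivery target that challenges the player with a random key prompt as they pass.
; An outer TriggerZone picks the key, reveals the KeyTrigger and shows the key on a popup widget, which turns toward the player every tick.
; KeyTrigger passes the key and delivery location to BP_PlayerCharacter.
; Leaving it resets the player's key state and damages health if neither a correct nor wrong key was pressed.
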(event OnComponentBeginOverlap(TriggerZone)
  (params (OverlappedComponent :type Primitive%20Component%20Object%20Reference) (OtherActor :type Actor%20Object%20Reference) (OtherComp :type Primitive%20Component%20Object%20Reference) (OtherBodyIndex :type Integer) (bFromSweep :type Boolean) (SweepResult :type Hit%20Result%20Structure%20%28by%20ref%29))
  (bind _widget (Variables|Default|GetWidget))
  (bind _asbp_player_character (Utilities|Casting|CastToBP_PlayerCharacter OtherActor))
  (Variables|Default|SetPCharacter _asbp_player_character)
  (Development|SetHiddeninGame _widget false false)
  (Development|SetHiddeninGame (Variables|Default|GetKeyTrigger) false false)
  (bind _returnvalue (Class|House|GetRandomKey))
  (bind _output_get (Variables|Default|SetCurrentKey _returnvalue))
  (bind _aswbp_key_pop_up (Utilities|Casting|CastToWBP_KeyPopUp (UserInterface|GetWidget _widget)))
  (Default|UpdateKeyUI _aswbp_key_pop_up _output_get))

(event OnComponentEndOverlap(KeyTrigger)
  (params (OverlappedComponent :type Primitive%20Component%20Object%20Reference) (OtherActor :type Actor%20Object%20Reference) (OtherComp :type Primitive%20Component%20Object%20Reference) (OtherBodyIndex :type Integer))
  (bind _asbp_player_character (Utilities|Casting|CastToBP_PlayerCharacter OtherActor))
  (Variables|/Script/LDJAM.PlayerCharacter|SetbInZone _asbp_player_character false)
  (if (or (Variables|/Script/LDJAM.PlayerCharacter|GetbKeyPressed _asbp_player_character) (Variables|/Script/LDJAM.PlayerCharacter|GetBWrongKeyPressed _asbp_player_character))
    _
    (else
      (Class|PlayerCharacter|DamageHealth _asbp_player_character)))
  (Variables|/Script/LDJAM.PlayerCharacter|SetbKeyPressed _asbp_player_character false)
  (Variables|/Script/LDJAM.PlayerCharacter|SetBWrongKeyPressed _asbp_player_character false))

(event OnComponentBeginOverlap(KeyTrigger)
  (params (OverlappedComponent :type Primitive%20Component%20Object%20Reference) (OtherActor :type Actor%20Object%20Reference) (OtherComp :type Primitive%20Component%20Object%20Reference) (OtherBodyIndex :type Integer) (bFromSweep :type Boolean) (SweepResult :type Hit%20Result%20Structure%20%28by%20ref%29))
  (bind _asbp_player_character (Utilities|Casting|CastToBP_PlayerCharacter OtherActor))
  (Class|PlayerCharacter|UpdateDeliveryData _asbp_player_character (Variables|Default|GetCurrentKey) (Transformation|GetWorldLocation (Variables|Default|GetDeliveryLocation)) true)
  (Development|PrintString "Hello"))

(event EventTick
  (params (DeltaSeconds :type Float%20%28single-precision%29))
  (Transformation|SetWorldRotation (Variables|Default|GetWidget) (Math|Rotator|FindLookatRotation (Transformation|GetWorldLocation (Variables|Default|GetWidget)) (Transformation|GetWorldLocation (Variables|/Script/Engine.Character|GetMesh (Game|GetPlayerCharacter 0)))) false false))

(fn ConstructionScript)